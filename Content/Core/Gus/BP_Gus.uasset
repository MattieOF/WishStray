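; Gus is a character that throws beer bottles at the player and, when exploded, brings up the W_Done end screen.
; While active, Tick derives Morale from player experience against the game mode's total item weight, deactivating Gus when it runs low, and turns him toward the player mid-throw.
; Throw functions attach a physics bottle to his hand, launch it with distance-scaled impulse, and delay its pawn collision.
; Explode swaps the mesh for a crumbling Geometry Collection.
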(event Custom|SetBottleCollisionInTime
  (params (Time :type Float%20%28double-precision%29))
  (bind _bottle (Variables|Default|GetBottle))
  (bind _meshcomp (Variables|/Script/WishStray.BreakableObject|GetMeshComp _bottle))
  (Utilities|FlowControl|Delay Time)
  (Utilities|IsValid _meshcomp
    (:Is%20Valid
      (Collision|SetCollisionResponsetoChannel _meshcomp "ECC_Pawn" "ECR_Block"))))

(event EventTick
  (params (DeltaSeconds :type Float%20%28single-precision%29))
  (bind _returnvalue (Transformation|GetActorRotation))
  (if (Variables|Default|GetActive)
    (bind _output_get (Variables|Default|SetMorale (- 1.0 (/ (Variables|/Script/WishStray.BengalCharacter|GetTotalExperience (.AsBengal%20Character (Utilities|Casting|CastToBengalCharacter (Game|Player|GetPlayerPawn 0)))) (Variables|/Script/WishStray.BengalGameMode|GetTotalItemWeight (.AsBengal%20Game%20Mode (Utilities|Casting|CastToBengalGameMode (Game|GetGameMode))))))))
    (if (< _output_get 0.08)
      (Variables|Default|SetActive false)
      (elif (Variables|Default|GetThrowing)
        (Transformation|SetActorRotation (Math|Rotator|MakeRotator (.roll _returnvalue) (.pitch _returnvalue) (.yaw (Math|Rotator|FindLookatRotation (Transformation|GetSocketLocation (Variables|Character|GetMesh) "Eyeline") (Transformation|GetActorLocation (Game|Player|GetPlayerPawn 0))))))))))

(fn ConstructionScript)

(fn BeginThrow
  (bind _returnvalue (Transformation|GetActorRotation))
  (bind _returnvalue_2 (Game|SpawnActorfromClass "/Game/Breakables/BRK_ThrownBeerBottle.BRK_ThrownBeerBottle_C" (Math|Transform|MakeTransform "0, 0, 0" "0, 0, 0" "1.000000,1.000000,1.000000") "Undefined" "MultiplyWithRoot" 0 0))
  (bind _output_get (Variables|Default|SetBottle _returnvalue_2))
  (Physics|SetSimulatePhysics (Variables|/Script/WishStray.BreakableObject|GetMeshComp _output_get) false)
  (Collision|SetCollisionEnabled (Variables|/Script/WishStray.BreakableObject|GetMeshComp _output_get) "NoCollision")
  (Transformation|AttachComponentToComponent _output_get (Variables|Character|GetMesh) "Hand" "KeepRelative" "KeepRelative" "KeepRelative" true)
  (Variables|Default|SetThrowing true)
  (Transformation|SetActorRotation (Math|Rotator|MakeRotator (.roll _returnvalue) (.pitch _returnvalue) (.yaw (Math|Rotator|FindLookatRotation (Transformation|GetSocketLocation (Variables|Character|GetMesh) "Eyeline") (Transformation|GetActorLocation (Game|Player|GetPlayerPawn 0)))))))

(fn EndThrow
  (bind _returnvalue (Game|Player|GetPlayerPawn 0))
  (bind _bottle (Variables|Default|GetBottle))
  (bind _bottle_2 (Variables|Default|GetBottle))
  (bind _returnvalue_2 (Transformation|GetActorLocation _returnvalue))
  (bind _returnvalue_3 (Transformation|GetActorLocation _bottle))
  (bind _meshcomp (Variables|/Script/WishStray.BreakableObject|GetMeshComp _bottle_2))
  (bind _returnvalue_4 (- _returnvalue_2 _returnvalue_3))
  (Transformation|DetachFromActor _bottle_2 "KeepWorld" "KeepWorld" "KeepWorld")
  (Collision|SetCollisionResponsetoChannel _meshcomp "ECC_Pawn" "ECR_Ignore")
  (Collision|SetCollisionEnabled _meshcomp "QueryAndPhysics")
  (Physics|SetSimulatePhysics _meshcomp true)
  (Physics|AddImpulse _meshcomp (* (Math|Vector|Normalize _returnvalue_4) (* (Math|Vector|VectorLength _returnvalue_4) 2.1)) "None" true)
  (CallFunction|SetBottleCollisioninTime 0.2))

(fn FullyEndThrow
  (Variables|Default|SetThrowing false))

(fn Explode
  (bind _returnvalue (Game|GetPlayerController 0))
  (bind _returnvalue_2 (AddComponent|AddGeometryCollectionComponent false (Math|Transform|MakeTransform "0.000000,0.000000,-460.000000" "0, 0, 0" "0.100000,0.100000,0.100000")))
  (Class|GeometryCollectionComponent|CrumbleActiveClusters _returnvalue_2)
  (Collision|SetCollisionEnabled (Variables|Collision|GetCapsuleComponent) "NoCollision")
  (Rendering|SetVisibility (Variables|Character|GetMesh) false false)
  (Input|SetInputModeUIOnly _returnvalue 0 "DoNotLock" true)
  (Variables|/Script/Engine.PlayerController|SetbShowMouseCursor _returnvalue true)
  (bind _returnvalue_3 (UserInterface|CreateWidget "/Game/UI/W_Done.W_Done_C"))
  (UserInterface|Viewport|AddtoViewport _returnvalue_3 0))